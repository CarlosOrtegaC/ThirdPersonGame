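; GM_Egipto is a game mode Blueprint that spawns and possesses the player character and manages a single held item.
; On BeginPlay it spawns BP_ThirdPersonCharacter at the first PlayerStart found, stores it as PlayerReference, has player controller 0 possess it and calls its Inicio.
; PickItem stores an item and destroys the picked actor only when none is held; DropItem is an empty stub.
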(event `self.ReceiveBeginPlay`
  (bind _outactors (`GameplayStatics.GetAllActorsOfClass` "/Script/Engine.PlayerStart"))
  (bind _returnvalue (`|SpawnActorFromClass` "/Game/ThirdPerson/Blueprints/BP_ThirdPersonCharacter.BP_ThirdPersonCharacter_C" (`self.GetTransform` (`|GetArrayItem` _outactors)) "Undefined" "MultiplyWithRoot" null null))
  (bind _output_get (set `self.PlayerReference` _returnvalue))
  (`Controller.Possess` (`GameplayStatics.GetPlayerController` 0) _output_get)
  (`/Game/ThirdPerson/Blueprints/BP_ThirdPersonCharacter.Inicio` _output_get))

(fn `DropItem`
  (params (InventoryItem :type "/Game/Blueprints/ST_PickUpItem Structure")))

(fn `PickItem`
  (params (InventoryItem :type "/Game/Blueprints/ST_PickUpItem Structure") (Target :type "Actor Object Reference"))
  (if (not (`self.HasItem`))
    (set `self.HasItem` true)
    (set `self.InventoryItem` InventoryItem)
    (`self.K2_DestroyActor` Target)))

(fn `UserConstructionScript`)