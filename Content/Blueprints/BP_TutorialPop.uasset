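; BP_TutorialPop is a trigger volume that pops up a tutorial widget the first time the player enters it.
; On BeginPlay it creates WG_Tutorial, adds it to the viewport and keeps it collapsed.
; Box overlaps by components tagged PlayerBody show the widget once, through a DoOnce, and collapse it on exit.
; The construction script sizes the Box from the BoxExtent variable.
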(event `self.ReceiveBeginPlay`
  (bind _returnvalue (`|CreateWidget` "/Game/Widgets/WG_Tutorial.WG_Tutorial_C" (`GameplayStatics.GetPlayerController` 0)))
  (bind _output_get (set `self.WGTutRef` _returnvalue))
  (`UserWidget.AddToViewport` _output_get 0)
  (`Widget.SetVisibility` _output_get "Collapsed"))

(event `self.Box.OnComponentBeginOverlap`
  (params (OverlappedComponent :type "PrimitiveComponent Object Reference") (OtherActor :type "Actor Object Reference") (OtherComp :type "PrimitiveComponent Object Reference") (OtherBodyIndex :type Integer) (bFromSweep :type Boolean) (SweepResult :type "HitResult Structure (by ref)"))
  (if (`ActorComponent.ComponentHasTag` OtherComp "PlayerBody")
    (`/Engine/EditorBlueprintResources/StandardMacros.DoOnce` false
      (:`Completed`
        (`Widget.SetVisibility` (`self.WGTutRef`) "Visible")))))

(event `self.Box.OnComponentEndOverlap`
  (params (OverlappedComponent :type "PrimitiveComponent Object Reference") (OtherActor :type "Actor Object Reference") (OtherComp :type "PrimitiveComponent Object Reference") (OtherBodyIndex :type Integer))
  (if (`ActorComponent.ComponentHasTag` OtherComp "PlayerBody")
    (`Widget.SetVisibility` (`self.WGTutRef`) "Collapsed")))

(fn `UserConstructionScript`
  (`BoxComponent.SetBoxExtent` (`self.Box`) (`self.Box Extent`) true))