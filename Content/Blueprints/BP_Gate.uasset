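; BP_Gate is a gate actor that rises vertically when its RemoteAction event fires.
; BeginPlay caches the Gate component's world location as the closed position.
; RemoteAction plays the GateTL timeline, whose GateDrive track lerps the gate up by GateRaisingHeight without sweeping.
; The timeline only plays forward, with no logic to lower the gate again.
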(event `self.ReceiveBeginPlay`
  (set `self.OriginalLocation` (`SceneComponent.K2_GetComponentLocation` (`self.Gate`))))

(event `/Game/Blueprints/BI_ItemComs.RemoteAction`
  (bind _originallocation (`self.OriginalLocation`))
  (bind (_direction _gatedrive) (`Timeline|GateTL`)
    (:`Update`
      (`SceneComponent.K2_SetWorldLocation` (`self.Gate`) (`KismetMathLibrary.VLerp` _originallocation (`KismetMathLibrary.MakeVector` (.x _originallocation) (.y _originallocation) (+ (.z _originallocation) (`self.GateRaisingHeight`))) _gatedrive) false false))))

(fn `UserConstructionScript`)