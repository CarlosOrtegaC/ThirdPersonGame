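; BP_Pickup is an interactable item pickup whose mesh is set from its ItemStats in the construction script.
; Focus and hide events toggle a widget, which, while visible, stays above the mesh bounds each tick and yaws toward the GM_Egipto game mode's player reference.
; Interacting passes ItemStats and the actor itself to the game mode's PickItem, which handles the pickup.
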(event `self.ReceiveBeginPlay`
  (set `self.As GM Egipto` (cast `/Game/Blueprints/GM_Egipto` (`GameplayStatics.GetGameMode`) :!pure true)))

(event `self.ReceiveTick`
  (params (DeltaSeconds :type "Float (single-precision)"))
  (bind _widget (`self.Widget`))
  (bind _staticmesh (`self.StaticMesh`))
  (bind (_returnvalue_roll _returnvalue_pitch _returnvalue_yaw) (`KismetMathLibrary.BreakRotator` (`KismetMathLibrary.FindLookAtRotation` (`SceneComponent.K2_GetComponentLocation` _widget) (`self.K2_GetActorLocation` (`/Game/Blueprints/GM_Egipto.PlayerReference` (`self.As GM Egipto`))))))
  (if (`SceneComponent.bVisible` _widget)
    (`SceneComponent.K2_SetWorldRotation` _widget (`KismetMathLibrary.MakeRotator` 0.0 0.0 _returnvalue_yaw) false false)
    (`SceneComponent.K2_SetWorldLocation` (`self.Widget`) (+ (`SceneComponent.K2_GetComponentLocation` _staticmesh) (`KismetMathLibrary.MakeVector` 0.0 0.0 (+ (.z (`.BoxExtent` (`KismetSystemLibrary.GetComponentBounds` _staticmesh))) 50.0))) false false)))

(event `/Game/Blueprints/BI_ItemComs.FocusTarget`
  (`SceneComponent.SetVisibility` (`self.Widget`) true false))

(event `/Game/Blueprints/BI_ItemComs.HideWidget`
  (`SceneComponent.SetVisibility` (`self.Widget`) false false))

(event `/Game/Blueprints/BI_ItemComs.InteractAction`
  (`/Game/Blueprints/GM_Egipto.PickItem` (cast `/Game/Blueprints/GM_Egipto` (`GameplayStatics.GetGameMode`) :!pure true) (`self.ItemStats`) self))

(fn `UserConstructionScript`
  (`StaticMeshComponent.SetStaticMesh` (`self.StaticMesh`) (`.ItemMesh_8_DE2B95F24670752BE23EBD9297EBB654` (break `/Game/Blueprints/ST_PickUpItem` (`self.ItemStats`)))))