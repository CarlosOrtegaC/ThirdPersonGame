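; BP_QuestGiver is an item-delivery quest NPC that talks to the player through GM_Egipto's quest widget.
; Box overlap toggles the widget and Niagara quest marker, while a QuestState enum selects dialogue and Spanish prompts.
; InteractAction advances reading and acceptance, swapping the marker effect, then compares the inventory item's name on delivery.
; The correct item completes the quest, is removed, and fires RemoteActionMessage on an optional TriggerActor.
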(event `self.ReceiveBeginPlay`
  (set `self.As GM Egipto` (cast `/Game/Blueprints/GM_Egipto` (`GameplayStatics.GetGameMode`) :!pure true)))

(event `self.Box.OnComponentBeginOverlap`
  (params (OverlappedComponent :type "PrimitiveComponent Object Reference") (OtherActor :type "Actor Object Reference") (OtherComp :type "PrimitiveComponent Object Reference") (OtherBodyIndex :type Integer) (bFromSweep :type Boolean) (SweepResult :type "HitResult Structure (by ref)"))
  ;[1 1 1] Eventos Overlap
  (if (`ActorComponent.ComponentHasTag` OtherComp "PlayerBody")
    (set `self.Overlaping` true)
    (`self.InteractTextIntro`)
    (`/Game/Blueprints/GM_Egipto.AddQuestToViewport` (`self.As GM Egipto`))
    (`self.PlayIntroMsg`)
    (`SceneComponent.SetVisibility` (`self.Niagara`) false false)))

(event `self.Box.OnComponentEndOverlap`
  (params (OverlappedComponent :type "PrimitiveComponent Object Reference") (OtherActor :type "Actor Object Reference") (OtherComp :type "PrimitiveComponent Object Reference") (OtherBodyIndex :type Integer))
  (bind _as_gm_egipto (`self.As GM Egipto`))
  ;[1 1 1] Eventos Overlap
  (if (`ActorComponent.ComponentHasTag` OtherComp "PlayerBody")
    (set `self.Overlaping` false)
    (`/Game/Widgets/WG_QuestMsg.Stop` (`/Game/Blueprints/GM_Egipto.WGQuestRef` _as_gm_egipto))
    (`/Game/Blueprints/GM_Egipto.RemoveQuestFromVP` _as_gm_egipto)
    (switch `/Game/Blueprints/E_QuestState` (`self.QuestState`)
      (:`NewEnumerator0`
        _)
      (:`NewEnumerator1`
        (set `self.QuestState` "NewEnumerator0"))
      (:`NewEnumerator2`
        (set `self.QuestState` "NewEnumerator3"))
      (:`NewEnumerator3`
        _))
    (`SceneComponent.SetVisibility` (`self.Niagara`) true false)))

(event `/Game/Blueprints/BI_ItemComs.InteractAction`
  (bind _playeracceptmessage (`/Game/Widgets/WG_QuestMsg.PlayerAcceptMessage` (`/Game/Blueprints/GM_Egipto.WGQuestRef` (`self.As GM Egipto`))))
  (if true
    (switch `/Game/Blueprints/E_QuestState` (`self.QuestState`)
      (:`NewEnumerator0`
        (`/Game/Widgets/WG_QuestMsg.Play` (`/Game/Blueprints/GM_Egipto.WGQuestRef` (`self.As GM Egipto`)) self (`self.MessageReading`))
        (set `self.QuestState` "NewEnumerator1")
        (`TextBlock.SetText` _playeracceptmessage "Pulsa E para Aceptar"))
      (:`NewEnumerator1`
        (`/Game/Widgets/WG_QuestMsg.Play` (`/Game/Blueprints/GM_Egipto.WGQuestRef` (`self.As GM Egipto`)) self (`self.MessageAccept`))
        (set `self.QuestState` "NewEnumerator2")
        (`TextBlock.SetText` _playeracceptmessage "")
        (`NiagaraComponent.SetAsset` (`self.Niagara`) "/Game/QuestMark/QuestMark2_FX.QuestMark2_FX" true))
      (:`NewEnumerator2`
        (`TextBlock.SetText` _playeracceptmessage "" :!label _label)
        (`self.PlayMessageDeliver`)
        (`self.CheckIfSolved`))
      (:`NewEnumerator3`
        (goto _label)))))

(fn `CheckIfSolved`
  (bind _triggeractor (`self.TriggerActor`))
  (if (`.CorrectItem` (`self.ItemCheck`))
    (set `self.QuestState` "NewEnumerator4")
    (`/Game/Blueprints/GM_Egipto.RemoveItem` (`self.As GM Egipto`))
    (`/Engine/EditorBlueprintResources/StandardMacros.IsValid` _triggeractor
      (:`Is Valid`
        (message `/Game/Blueprints/BI_ItemComs.RemoteAction` _triggeractor)))))

(fn `InteractTextIntro`
  (bind _playeracceptmessage (`/Game/Widgets/WG_QuestMsg.PlayerAcceptMessage` (`/Game/Blueprints/GM_Egipto.WGQuestRef` (`self.As GM Egipto`))))
  (switch `/Game/Blueprints/E_QuestState` (`self.QuestState`)
    (:`NewEnumerator0`
      (`TextBlock.SetText` _playeracceptmessage "Pulsa E para continuar" :!label _label))
    (:`NewEnumerator1`
      (`TextBlock.SetText` _playeracceptmessage "" :!label _label_2))
    (:`NewEnumerator2`
      (goto _label_2))
    (:`NewEnumerator3`
      (if (`self.ItemCheck`)
        (goto _label)
        (else
          (`TextBlock.SetText` _playeracceptmessage "Pulsa E para entregar el objeto"))))
    (:`NewEnumerator4`
      (goto _label_2))))

(fn `ItemCheck`
  (returns (NoItem :type Boolean) (CorrectItem :type Boolean))
  (bind _itemname (break `/Game/Blueprints/ST_PickUpItem` (`/Game/Blueprints/GM_Egipto.InventoryItem` (`self.As GM Egipto`))))
  (return (== _itemname "None") (== _itemname (`self.CorrectItem`))))

(fn `PlayIntroMsg`
  (`/Game/Widgets/WG_QuestMsg.Play` (`/Game/Blueprints/GM_Egipto.WGQuestRef` (`self.As GM Egipto`)) self (select `/Game/Blueprints/E_QuestState` (`self.QuestState`) :`NewEnumerator0` (`self.MessageBegin`) :`NewEnumerator3` (`self.MessagePending`) :`NewEnumerator4` (`self.MessageComplete`))))

(fn `PlayMessageDeliver`
  (bind (_noitem _correctitem) (`self.ItemCheck`))
  (`/Game/Widgets/WG_QuestMsg.Play` (`/Game/Blueprints/GM_Egipto.WGQuestRef` (`self.As GM Egipto`)) self (`KismetMathLibrary.SelectString` (`self.MessageNoItem`) (`KismetMathLibrary.SelectString` (`self.MessageCorrectItem`) (`self.MessageWrongItem`) _correctitem) _noitem)))

(fn `UserConstructionScript`
  (`BoxComponent.SetBoxExtent` (`self.Box`) (`self.BoxExtent`) true))