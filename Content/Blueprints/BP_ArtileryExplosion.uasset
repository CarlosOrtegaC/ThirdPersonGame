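; BP_ArtileryExplosion is a one-shot interactable actor that sets off a particle effect and the ending sequence.
; Focus events show or hide a prompt widget, which yaws each tick toward the player reference held by GM_Egipto while visible.
; On first interaction it activates the particles, hides the widget, disables player input and plays the EndingSequence level sequence, with an Activated flag blocking further prompts and triggers.
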(event `self.ReceiveBeginPlay`
  (set `self.As GM Egipto` (cast `/Game/Blueprints/GM_Egipto` (`GameplayStatics.GetGameMode`) :!pure true)))

(event `self.ReceiveTick`
  (params (DeltaSeconds :type "Float (single-precision)"))
  (bind _widget (`self.Widget`))
  (bind (_returnvalue_roll _returnvalue_pitch _returnvalue_yaw) (`KismetMathLibrary.BreakRotator` (`KismetMathLibrary.FindLookAtRotation` (`SceneComponent.K2_GetComponentLocation` _widget) (`self.K2_GetActorLocation` (`/Game/Blueprints/GM_Egipto.PlayerReference` (`self.As GM Egipto`))))))
  (if (`SceneComponent.bVisible` _widget)
    (`SceneComponent.K2_SetWorldRotation` _widget (`KismetMathLibrary.MakeRotator` 0.0 0.0 _returnvalue_yaw) false false)))

(event `/Game/Blueprints/BI_ItemComs.FocusTarget`
  (if (not (`self.Activated`))
    (`SceneComponent.SetVisibility` (`self.Widget`) true false)))

(event `/Game/Blueprints/BI_ItemComs.HideWidget`
  (`SceneComponent.SetVisibility` (`self.Widget`) false false))

(event `/Game/Blueprints/BI_ItemComs.InteractAction`
  (if (not (`self.Activated`))
    (`ActorComponent.Activate` (`self.ParticleSystem`) true)
    (set `self.Activated` true)
    (`SceneComponent.SetVisibility` (`self.Widget`) false false)
    (`self.DisableInput` (`/Game/Blueprints/GM_Egipto.PlayerReference` (`self.As GM Egipto`)) (`GameplayStatics.GetPlayerController` 0))
    (bind (_outactor _returnvalue) (`LevelSequencePlayer.CreateLevelSequencePlayer` "/Game/EndingSequence.EndingSequence"))
    (`MovieSceneSequencePlayer.Play` _returnvalue)))

(fn `UserConstructionScript`)